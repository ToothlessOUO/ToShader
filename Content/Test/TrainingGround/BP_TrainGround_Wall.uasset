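; Training ground wall actor that builds a tiled wall from a configurable width and height.
; The construction script adds one instance per grid cell to the Wall instanced mesh, spaced by FloorSize, roughly centered on local Y and stacked along Z.
; Each tile gets an unseeded random quarter-turn yaw, so the pattern can change whenever construction reruns.
; The event graph holds no active logic.
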(event EventBeginPlay)

(event Collision|EventActorBeginOverlap
  (params (OtherActor :type Actor%20Object%20Reference)))

(event EventTick
  (params (DeltaSeconds :type Float%20%28single-precision%29)))

(fn ConstructionScript
  (bind _width (Variables|Default|GetWidth))
  (bind _floorsize (Variables|Default|GetFloorSize))
  (for _index (range 1 _width)
    (for _index_2 (range 1 (Variables|Default|GetHeight))
      (Components|InstancedStaticMesh|AddInstance (Variables|Default|GetWall) (Math|Transform|MakeTransform (Math|Vector|MakeVector 0.0 (* (+ (- _index (/ _width 2)) -1) _floorsize) (- (* _index_2 _floorsize) 1e+02)) (Math|Rotator|MakeRotator 0.0 0.0 (Math|Conversions|ToFloat(Integer) (* 90 (Math|Float|Floor (Math|Random|RandomFloatinRange -2.0 2.0))))) "1.000000,1.000000,1.000000") false))))