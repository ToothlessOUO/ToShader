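; BP_Ellen is a test Blueprint for the Ellen character, assembled from multiple mesh components.
; Its construction script makes Body1 the leader pose component for the weapon, face, eye, second body, mask and outline meshes, forcing an update so they follow its animation.
; Tick only calls the parent implementation, and the BeginPlay and overlap events are disabled placeholders.
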(event EventBeginPlay)

(event Collision|EventActorBeginOverlap
  (params (OtherActor :type Actor%20Object%20Reference)))

(event EventTick
  (params (DeltaSeconds :type Float%20%28single-precision%29))
  (|CallParentFunction DeltaSeconds))

(fn ConstructionScript
  (Utilities|FlowControl|Sequence
    (:then_1
      (Components|SkinnedMesh|SetLeaderPoseComponent (Variables|Default|GetWeapon) (Variables|Default|GetBody1) true true))))