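; BP_TrainGround is a procedural floor generator for a test training ground, built entirely in the construction script.
; It lays a Width by Height grid of Floors instances spaced by FloorSize, roughly centered on the actor.
; Each tile gets a random quarter-turn yaw, re-rolled whenever construction reruns, to vary the surface.
; Lights instances are added on tiles where both grid indices are odd; the event graph is unused.
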(event EventBeginPlay)

(event Collision|EventActorBeginOverlap
  (params (OtherActor :type Actor%20Object%20Reference)))

(event EventTick
  (params (DeltaSeconds :type Float%20%28single-precision%29)))

(fn ConstructionScript
  (bind _width (Variables|Default|GetWidth))
  (bind _height (Variables|Default|GetHeight))
  (bind _floorsize (Variables|Default|GetFloorSize))
  (for _index (range 1 _width)
    (for _index_2 (range 1 _height)
      (Components|InstancedStaticMesh|AddInstance (Variables|Default|GetFloors) (Math|Transform|MakeTransform (Math|Vector|MakeVector (* (+ (- _index (/ _width 2)) -1) _floorsize) (* (+ (- _index_2 (/ _height 2)) -1) _floorsize) 0.0) (Math|Rotator|MakeRotator 0.0 0.0 (Math|Conversions|ToFloat(Integer) (* 90 (Math|Float|Floor (Math|Random|RandomFloatinRange -2.0 2.0))))) "1.000000,1.000000,1.000000") false)
      (if (and (== (Math|Integer|%(Integer) _index 2) 1) (== (Math|Integer|%(Integer) _index_2 2) 1))
        (Components|InstancedStaticMesh|AddInstance (Variables|Default|GetLights) (Math|Transform|MakeTransform (Math|Vector|MakeVector (* (+ (- _index (/ _width 2)) -1) _floorsize) (* (+ (- _index_2 (/ _height 2)) -1) _floorsize) 0.0) "0, 0, 0" "1.000000,1.000000,1.000000") false)))))