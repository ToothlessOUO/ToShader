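; BP_Test is a test actor that triggers a shader effect through its ToShader member.
; Its ApplyEffect event calls ApplyNewEffect on ToShader, waits briefly, then calls it again.
; Disconnected leftover chains experiment with driving static mesh custom primitive data, directly or from a timeline, and setting a texture array on a dynamic material instance; none of them run.
; Tick only calls the parent, and the construction script is empty.
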(event Custom|ApplyEffect
  (bind _toshader (Variables|Default|GetToShader))
  (Class|ToShaderComponent|ApplyNewEffect _toshader)
  (Utilities|FlowControl|Delay 1.0)
  (Class|ToShaderComponent|ApplyNewEffect _toshader))

(event EventBeginPlay)

(event Collision|EventActorBeginOverlap
  (params (OtherActor :type Actor%20Object%20Reference)))

(event EventTick
  (params (DeltaSeconds :type Float%20%28single-precision%29))
  (|CallParentFunction DeltaSeconds))

(fn ConstructionScript)